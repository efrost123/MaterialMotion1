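; Sphere actor Blueprint that tints its mesh through the material's "base_color" parameter based on a vector input axis.
; Each Tick remaps axis X and Y from -2..2 to 0..1 as red and blue, keeps green, and prints both values.
; The construction script sets blue from BaseColor, and two functions update red or blue individually.
; Tick and both functions call CreateDynamicMaterialInstance on every run.
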(event `self.ReceiveTick`
  (params (DeltaSeconds :type "Float (single-precision)"))
  (bind _returnvalue (/ (- (.x (`self.GetInputVectorAxisValue`)) -2.0) 4.0))
  (bind _returnvalue_2 (/ (- (.y (`self.GetInputVectorAxisValue`)) -2.0) 4.0))
  (bind _returnvalue_3 (`PrimitiveComponent.CreateDynamicMaterialInstance` (`self.StaticMeshComponent0`) 0 "/Game/NewMaterial.NewMaterial" "None"))
  (bind _returnvalue_4 (`MaterialInstanceDynamic.K2_GetVectorParameterValue` _returnvalue_3 "base_color"))
  (`MeshComponent.SetVectorParameterValueOnMaterials` (`self.StaticMeshComponent0`) "base_color" (`KismetMathLibrary.Conv_LinearColorToVector` (`KismetMathLibrary.MakeColor` _returnvalue (`.G` (break `LinearColor` _returnvalue_4)) _returnvalue_2)))
  (`KismetSystemLibrary.PrintString` (`KismetTextLibrary.Conv_TextToString` (`|FormatText` "x: {xValue} y:{yValue}" _returnvalue _returnvalue_2)) true true (struct :`R` 1.0 :`G` 0.161928 :`B` 0.967771 :`A` 1.0) 0.5))

(fn `UpdateBlueComponent`
  (params (BlueLevelValue :type "Float (double-precision)"))
  (bind _returnvalue (`PrimitiveComponent.CreateDynamicMaterialInstance` (`self.StaticMeshComponent0`) 0 "/Game/NewMaterial.NewMaterial" "None"))
  (bind _returnvalue_2 (`MaterialInstanceDynamic.K2_GetVectorParameterValue` _returnvalue "base_color"))
  (bind (_r _g _b _a) (break `LinearColor` _returnvalue_2))
  (`MeshComponent.SetVectorParameterValueOnMaterials` (`self.StaticMeshComponent0`) "base_color" (`KismetMathLibrary.Conv_LinearColorToVector` (`KismetMathLibrary.MakeColor` _r _g BlueLevelValue _a))))

(fn `UpdateRedComponent`
  (params (RedLevelValue :type "Float (double-precision)"))
  (bind _returnvalue (`PrimitiveComponent.CreateDynamicMaterialInstance` (`self.StaticMeshComponent0`) 0 "/Game/NewMaterial.NewMaterial" "None"))
  (bind _returnvalue_2 (`MaterialInstanceDynamic.K2_GetVectorParameterValue` _returnvalue "base_color"))
  (bind (_r _g _b _a) (break `LinearColor` _returnvalue_2))
  (`MeshComponent.SetVectorParameterValueOnMaterials` (`self.StaticMeshComponent0`) "base_color" (`KismetMathLibrary.Conv_LinearColorToVector` (`KismetMathLibrary.MakeColor` RedLevelValue _g _b _a))))

(fn `UserConstructionScript`
  (bind _returnvalue (`MaterialInstanceDynamic.K2_GetVectorParameterValue` (stale _returnvalue_2) "base_color"))
  (bind _returnvalue_2 (`PrimitiveComponent.CreateDynamicMaterialInstance` (`self.StaticMeshComponent0`) 0 "/Game/NewMaterial.NewMaterial" "None"))
  (bind (_r _g _b _a) (break `LinearColor` _returnvalue))
  (`MaterialInstanceDynamic.SetVectorParameterValue` _returnvalue_2 "base_color" (`KismetMathLibrary.MakeColor` _r _g (`self.BaseColor`) _a)))